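; GM_Main is the game mode that tracks level progression, enemy count and score, and relays game events to the HUD.
; BeginPlay creates WBP_HUD and shows the mouse cursor.
; StartLevel sets remaining enemies from EnemyCount times Level, and RemoveEnemy flags the level finished and increments Level when none remain.
; Other events forward fades, life loss, weapon changes, win and lose to the HUD, while AddPoints accumulates score.
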(event `self.ReceiveBeginPlay`
  (bind _returnvalue (`|CreateWidget` "/Game/Blueprints/Widget/WBP_HUD.WBP_HUD_C"))
  (bind _output_get (set `self.HUDReference` _returnvalue))
  (`UserWidget.AddToViewport` _output_get 0)
  (set `PlayerController.bShowMouseCursor` true (`GameplayStatics.GetPlayerController` 0)))

(event `StartLevel`
  (set `self.EnemiesRemaining` (* (`self.EnemyCount`) (`self.Level`)))
  (set `self.finishedLevel` false)
  (`self.UseFadeIn`))

(event `RestartLevel`
  (set `self.finishedLevel` false)
  (`self.UseFadeIn`))

(event `RemoveEnemy`
  (bind _output_get (set `self.EnemiesRemaining` (- (`self.EnemiesRemaining`) 1)))
  (if (<= _output_get 0)
    (set `self.finishedLevel` true)
    (set `self.Level` (+ (`self.Level`) 1))))

(event `AddPoints`
  (params (Added :type Integer))
  (set `self.Points` (+ Added (`self.Points`))))

(event `UseFadeIn`
  (`/Game/Blueprints/Widget/WBP_HUD.ToggleFadeIn` (`self.HUDReference`) false))

(event `UseFadeOutNextLevel`
  (bind _hudreference (`self.HUDReference`))
  (`/Game/Blueprints/Widget/WBP_HUD.ChangeLevel` _hudreference)
  (`/Game/Blueprints/Widget/WBP_HUD.ToggleFadeIn` _hudreference true))

(event `UseFadeOutRestartLevel`
  (`/Game/Blueprints/Widget/WBP_HUD.ToggleFadeIn` (`self.HUDReference`) true))

(event `Lose`
  (`/Game/Blueprints/Widget/WBP_HUD.Lose` (`self.HUDReference`)))

(event `LoseLife`
  (`/Game/Blueprints/Widget/WBP_HUD.LoseHeart` (`self.HUDReference`)))

(event `SetCurrentWeapon`
  (params (CurrentWeapon :type "/Game/Blueprints/Weapons/BP_Weapon Class Reference"))
  (`/Game/Blueprints/Widget/WBP_HUD.SetCurrentWeapon` (`self.HUDReference`) CurrentWeapon))

(event `Win`
  (`/Game/Blueprints/Widget/WBP_HUD.Win` (`self.HUDReference`)))

(fn `UserConstructionScript`)