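; BP_Launcher is a launcher weapon that spawns one projectile of its Bullet class at the ShootingPoint transform per accepted StartFire.
; A CanShoot flag gates firing: it is set on BeginPlay and cleared when a shot spawns.
; Each shot sets a looping FireRate timer on ResetFire, which restores the flag without firing again.
; StopFire only clears the flag and leaves that timer running, so the next tick re-enables shooting.
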(event `self.ReceiveBeginPlay`
  (`parent.ReceiveBeginPlay`)
  (set `self.canShoot` true))

(event `ResetFire`
  (set `self.canShoot` true))

(event `/Game/Blueprints/Weapons/IFire.StartFire`
  (if (`self.canShoot`)
    (set `self.canShoot` false)
    (`|SpawnActorFromClass` "/Game/Blueprints/Weapons/Launcher/Bullet.Bullet_C" (`SceneComponent.K2_GetComponentToWorld` (`self.ShootingPoint`)) "Undefined" "MultiplyWithRoot" null null)
    (`KismetSystemLibrary.K2_SetTimerDelegate` (delegate `ResetFire`) (`self.FireRate`) true)))

(event `/Game/Blueprints/Weapons/IFire.StopFire`
  (set `self.canShoot` false))

(fn `UserConstructionScript`
  (`parent.UserConstructionScript`))