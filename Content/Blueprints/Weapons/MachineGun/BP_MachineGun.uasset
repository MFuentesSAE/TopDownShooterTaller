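; Machine gun weapon Blueprint that fires hitscan shots toward the mouse cursor and kills zombies it hits.
; StartFire, gated by CanShoot, shakes the camera, spawns a Niagara tracer and line traces out to Range, calling Die on any BP_Zombie hit.
; Aim uses the cursor's impact point flattened to muzzle height, keeping shots horizontal.
; A looping FireRate timer re-enables CanShoot, while StopFire clears it without stopping that timer.
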(event `self.ReceiveBeginPlay`
  (`parent.ReceiveBeginPlay`)
  (set `self.canShoot` true))

(event `ResetFire`
  (set `self.canShoot` true))

(event `/Game/Blueprints/Weapons/IFire.StartFire`
  (bind (_returnvalue_x _returnvalue_y _returnvalue_z) (`KismetMathLibrary.BreakVector` (`SceneComponent.K2_GetComponentLocation` (`self.ShootingPoint`))))
  (bind (_bblockinghit _binitialoverlap _time _distance _location _impactpoint) (`GameplayStatics.BreakHitResult` (`PlayerController.GetHitResultUnderCursorByChannel` (`GameplayStatics.GetPlayerController` 0) "TraceTypeQuery1" true)))
  (bind _returnvalue (`KismetMathLibrary.MakeVector` _returnvalue_x _returnvalue_y _returnvalue_z))
  (bind _returnvalue_2 (+ _returnvalue (* (`KismetMathLibrary.Normal` (- (`KismetMathLibrary.MakeVector` (.x _impactpoint) (.y _impactpoint) _returnvalue_z) _returnvalue)) (`self.Range`))))
  (if (`self.canShoot`)
    (`PlayerController.ClientStartCameraShake` :`self` (`GameplayStatics.GetPlayerController` 0) :`Shake` "/Game/Blueprints/CameraShake/BP_CameraShake_Shooting.BP_CameraShake_Shooting_C")
    (set `self.canShoot` false)
    (bind _returnvalue_3 (`NiagaraFunctionLibrary.SpawnSystemAtLocation` "/Game/Realistic_Starter_VFX_Pack_Vol2/Particles/NS_BulletTracer.NS_BulletTracer"))
    (`NiagaraComponent.SetVariableVec3` _returnvalue_3 "Start" _returnvalue)
    (`NiagaraComponent.SetVariableVec3` _returnvalue_3 "Target" _returnvalue_2)
    (bind _outhit (`KismetSystemLibrary.LineTraceSingle` _returnvalue _returnvalue_2 "TraceTypeQuery1"))
    (`KismetSystemLibrary.K2_SetTimerDelegate` (delegate `ResetFire`) (`self.FireRate`) true)
    (bind (_bblockinghit_2 _binitialoverlap_2 _time_2 _distance_2 _location_2 _impactpoint_2 _normal _impactnormal _physmat _hitactor) (`GameplayStatics.BreakHitResult` _outhit))
    (if (`GameplayStatics.ObjectIsA` _hitactor "/Game/Blueprints/Enemys/BP_Zombie.BP_Zombie_C")
      (bind _asbp_zombie (cast `/Game/Blueprints/Enemys/BP_Zombie` _hitactor))
      (`/Game/Blueprints/Enemys/BP_Zombie.Die` _asbp_zombie))))

(event `/Game/Blueprints/Weapons/IFire.StopFire`
  (set `self.canShoot` false))

(fn `UserConstructionScript`
  (`parent.UserConstructionScript`))