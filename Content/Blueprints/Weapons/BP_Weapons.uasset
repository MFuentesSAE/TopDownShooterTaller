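; Player weapon manager that handles temporary weapon and shield pickups and forwards shoot and stop-shooting calls to the current weapon.
; Weapons spawn attached to the player's WeaponPlacement and are reported to GM_Main, starting with the default.
; A non-default weapon reverts to the default after a timer, which restarts on each such equip.
; Shields attach at ShieldPlacement and are destroyed by their own restartable timer.
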(event `self.ReceiveBeginPlay`
  (bind _asbp_player (cast `/Game/Blueprints/Player/BP_Player` (`self.GetOwner`)))
  (set `self.playerRef` _asbp_player)
  (bind _asgm_main (cast `/Game/Input/GM_Main` (`GameplayStatics.GetGameMode`)))
  (set `self.GameMode` _asgm_main)
  (`self.ReturnToDerfaultWeapon`))

(event `EquipNewWeapon`
  (params (newWeapon :type "/Game/Blueprints/Weapons/BP_Weapon Class Reference"))
  (bind _currentweapon (`self.CurrentWeapon`))
  (bind _weaponplacement (`/Game/Blueprints/Player/BP_Player.WeaponPlacement` (`self.playerRef`)))
  ; Equip New Weapon
  (if (!= newWeapon (`self.DefaultWeapon`))
    (`/Engine/EditorBlueprintResources/StandardMacros.IsValid` _currentweapon
      (:`Is Valid`
        (`Actor.K2_DestroyActor` _currentweapon))
      (:`Is Not Valid`
        _))
    (bind _returnvalue (`|SpawnActorFromClass` newWeapon (`SceneComponent.K2_GetComponentToWorld` _weaponplacement) "AlwaysSpawn" "MultiplyWithRoot" null null))
    (bind _output_get (set `self.CurrentWeapon` _returnvalue))
    (`Actor.K2_AttachToComponent` _output_get _weaponplacement "None" "KeepWorld" "KeepWorld" "KeepWorld" true)
    (`KismetSystemLibrary.K2_ClearAndInvalidateTimerHandle` (`self.WeaponTimer`))
    (bind _returnvalue_2 (`KismetSystemLibrary.K2_SetTimerDelegate` (delegate `ReturnToDerfaultWeapon`) 10.0))
    (set `self.WeaponTimer` _returnvalue_2)
    (`/Game/Input/GM_Main.SetCurrentWeapon` (`self.GameMode`) newWeapon)))

(event `ReturnToDerfaultWeapon`
  (bind _defaultweapon (`self.DefaultWeapon`))
  (bind _currentweapon (`self.CurrentWeapon`))
  (bind _weaponplacement (`/Game/Blueprints/Player/BP_Player.WeaponPlacement` (`self.playerRef`)))
  ; Return To Default Weapon
  (`/Engine/EditorBlueprintResources/StandardMacros.IsValid` _currentweapon
    (:`Is Valid`
      (`Actor.K2_DestroyActor` _currentweapon))
    (:`Is Not Valid`
      _))
  (bind _returnvalue (`|SpawnActorFromClass` _defaultweapon (`SceneComponent.K2_GetComponentToWorld` _weaponplacement) "AlwaysSpawn" "MultiplyWithRoot" null null))
  (bind _output_get (set `self.CurrentWeapon` _returnvalue))
  (`Actor.K2_AttachToComponent` _output_get _weaponplacement "None" "KeepWorld" "KeepWorld" "KeepWorld" true)
  (`/Game/Input/GM_Main.SetCurrentWeapon` (`self.GameMode`) _defaultweapon))

(event `Shoot`
  ; Shoot
  (if (`KismetSystemLibrary.IsValid` (`self.CurrentWeapon`))
    (`/Game/Blueprints/Weapons/BP_Weapon.Shoot` (`self.CurrentWeapon`))))

(event `StopShooting`
  ; Stop Shooting
  (if (`KismetSystemLibrary.IsValid` (`self.CurrentWeapon`))
    (`/Game/Blueprints/Weapons/BP_Weapon.StopShooting` (`self.CurrentWeapon`))))

(event `PickUpShield`
  (bind _playerref (`self.playerRef`))
  (bind _shieldplacement (`/Game/Blueprints/Player/BP_Player.ShieldPlacement` _playerref))
  ; AttachShield
  (bind _returnvalue (`|SpawnActorFromClass` "/Game/Blueprints/Shield/Shield.Shield_C" (`SceneComponent.K2_GetComponentToWorld` _shieldplacement) "Undefined" "MultiplyWithRoot" _playerref null))
  (bind _output_get (set `self.CurrentShield` _returnvalue))
  (`Actor.K2_AttachToComponent` _output_get _shieldplacement "None" "KeepWorld" "KeepWorld" "KeepWorld" true)
  (`KismetSystemLibrary.K2_ClearAndInvalidateTimerHandle` (`self.ShieldTimer`))
  (bind _returnvalue_2 (`KismetSystemLibrary.K2_SetTimerDelegate` (delegate `RemoveShield`) 10.0))
  (set `self.ShieldTimer` _returnvalue_2))

(event `RemoveShield`
  ; Remove Shield
  (`Actor.K2_DestroyActor` (`self.CurrentShield`)))