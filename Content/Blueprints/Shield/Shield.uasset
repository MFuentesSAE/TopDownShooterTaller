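; Shield actor that kills any BP_Zombie overlapping its Sphere by calling Die on it.
; While IsActive is set, Tick spins the Center component in local yaw at RotationSpeed, scaled by delta time.
; Despawn only hides the root and its children, leaving the actor, its collision and IsActive untouched.
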(event `self.ReceiveBeginPlay`)

(event `Despawn`
  (`SceneComponent.SetVisibility` (`self.DefaultSceneRoot`) false true))

(event `self.Sphere.OnComponentBeginOverlap`
  (params (OverlappedComponent :type "PrimitiveComponent Object Reference") (OtherActor :type "Actor Object Reference") (OtherComp :type "PrimitiveComponent Object Reference") (OtherBodyIndex :type Integer) (bFromSweep :type Boolean) (SweepResult :type "HitResult Structure (by ref)"))
  (if (`GameplayStatics.ObjectIsA` OtherActor "/Game/Blueprints/Enemys/BP_Zombie.BP_Zombie_C")
    (bind _asbp_zombie (cast `/Game/Blueprints/Enemys/BP_Zombie` OtherActor))
    (`/Game/Blueprints/Enemys/BP_Zombie.Die` _asbp_zombie)))

(event `self.ReceiveTick`
  (params (DeltaSeconds :type "Float (single-precision)"))
  (if (`self.isActive`)
    (`SceneComponent.K2_AddLocalRotation` (`self.Center`) (`KismetMathLibrary.MakeRotator` 0.0 0.0 (* (`GameplayStatics.GetWorldDeltaSeconds`) (`self.rotationSpeed`))) false false)))

(fn `UserConstructionScript`)